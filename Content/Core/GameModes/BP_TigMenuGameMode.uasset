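; Menu game mode that exposes level streaming and level travel events.
; A streaming graph wraps loading and unloading of sublevels by name or soft object reference, plus a direct open-level call.
; A separate open event requests a non-blocking unload of L_Main before opening the target level by reference.
; BeginPlay only prints a colored check-in message.
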(event Custom|OpenLevelByObjectReference
  (params (Level :type World%20Soft%20Object%20Reference) (bAbsolute :type Boolean) (Options :type String))
  (Class|GameplayStatics|UnloadStreamLevelbySoftObjectPtr "/Game/Art/Maps/L_Main.L_Main" false)
  (Game|OpenLevel(byObjectReference) Level bAbsolute Options))

(event EventBeginPlay
  (CallFunction|COut "BeginPlay" "Checking in." "(R=0.000000,G=1.000000,B=0.000000,A=1.000000)" false))

(event Custom|LoadLevelByName
  (params (LevelName :type Name :default "none") (bMakeVisibleAfterLoad :type Boolean) (bShouldBlockOnLoad :type Boolean))
  (Game|LoadStreamLevel(byName) LevelName bMakeVisibleAfterLoad bShouldBlockOnLoad))

(event Custom|UnloadLevelByName
  (params (LevelName :type Name) (bShouldBlockOnUnload :type Boolean))
  (Game|UnloadStreamLevel(byName) LevelName bShouldBlockOnUnload))

(event Custom|UnloadLevel
  (params (Level :type World%20Soft%20Object%20Reference) (bShouldBlockOnUnload :type Boolean))
  (Class|GameplayStatics|UnloadStreamLevelbySoftObjectPtr Level bShouldBlockOnUnload))

(event Custom|LoadLevel
  (params (Level :type World%20Soft%20Object%20Reference) (bMakeVisibleAfterLoad :type Boolean) (bShouldBlockOnLoad :type Boolean))
  (Class|GameplayStatics|LoadStreamLevelbySoftObjectPtr Level bMakeVisibleAfterLoad bShouldBlockOnLoad))

(event Custom|OpenLevel
  (params (Level :type World%20Soft%20Object%20Reference) (bAbsolute :type Boolean) (Options :type String))
  (Game|OpenLevel(byObjectReference) Level bAbsolute Options))

(fn ConstructionScript)