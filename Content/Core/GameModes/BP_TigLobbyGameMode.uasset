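; Lobby game mode that manages connected players, map settings, character selection and kicking before launching the match.
; It reads server info from the game instance, registers players on login and pushes lobby updates to player controllers through interface-style messages.
; Character changes respawn pawns at random spawn points, with an availability array tracking picks and updated on logout.
; Launch shows loading screens, then server-travels to a debug map chosen by MapID.
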(event Custom|OpenLevelByObjectReference
  (params (Level :type World%20Soft%20Object%20Reference) (bAbsolute :type Boolean) (Options :type String))
  ;[1 1 1] Kal's chopping block
  ;;[1 1 1] OpenLevelByObjectReference
  (Class|GameplayStatics|UnloadStreamLevelbySoftObjectPtr "/Game/Art/Maps/L_Main.L_Main" false)
  (Game|OpenLevel(byObjectReference) Level bAbsolute Options))

(event Custom|StartLoadingScreen
  ;[1 1 1] Shows loading screen and launches the game.
  (for _array_element (Variables|Default|GetConnectedPlayers)
    (bind _aslobbyplayercontroller (Class|BPILobbyPlayerController|LobbyPlayerControllerRef(Message) _array_element))
    (Class|BPIGameInstance|ShowLoadingScreen(Message) _aslobbyplayercontroller))
  (CallFunction|LaunchGame))

(event Custom|HostUpdateGameSettings
  (params (SelectedMapImage :type Texture%202D%20Object%20Reference%20%28by%20ref%29) (SelectedMapName :type Text%20%28by%20ref%29) (SelectedMapTime :type Text%20%28by%20ref%29) (MapID :type Integer))
  ;[1 1 1] HostUpdateGameSettings - Server has made changes to settings so update all the client's screens.
  (Variables|Default|SetSelectedMapImage SelectedMapImage)
  (Variables|Default|SetSelectedMapName SelectedMapName)
  (Variables|Default|SetSelectedMapTime SelectedMapTime)
  (Variables|Default|SetMapID MapID)
  (for _array_element (Variables|Default|GetConnectedPlayers)
    (bind _aslobbyplayercontroller (Class|BPILobbyPlayerController|LobbyPlayerControllerRef(Message) _array_element))
    (Default|UpdateLobbySettings _aslobbyplayercontroller (Variables|Default|GetSelectedMapImage) (Variables|Default|GetSelectedMapName) (Variables|Default|GetSelectedMapTime))))

(event Custom|PlayerKicked
  (params (PlayerID :type Integer))
  ;[1 1 1] Kick functionality
  ;;[1 1 1] PlayerKicked - Kick selected player from game session
  (bind _aslobbyplayercontroller (Class|BPILobbyPlayerController|LobbyPlayerControllerRef(Message) (Utilities|Array|Get(acopy) (Variables|Default|GetConnectedPlayers) PlayerID)))
  (Default|Kicked _aslobbyplayercontroller))

(event Custom|EveryoneUpdate
  (bind _connectedplayers (Variables|Default|GetConnectedPlayers))
  ;[1 1 1] Update all connected player's lobby widget information when called.
  (bind _output_get (Variables|Default|SetCurrentPlayers (Utilities|Array|Length (Variables|Default|GetConnectedPlayers))))
  (if (> _output_get 0)
    (Utilities|Array|Clear (Variables|Default|GetConnectedPlayersInfo))
    (for _array_element _connectedplayers
      (bind _aslobbyplayercontroller (Class|BPILobbyPlayerController|LobbyPlayerControllerRef(Message) _array_element))
      (Utilities|Array|AddUnique (Variables|Default|GetConnectedPlayersInfo) (Variables|/Game/Core/GameInstances/BP_TigGameInstance.BP_TigGameInstance_C|GetPlayers%20Info (Variables|Default|GetAs%20BP%20Tig%20Game%20Instance)))
      (Default|UpdateNumberOfPlayers _aslobbyplayercontroller (Variables|Default|GetCurrentPlayers) (Variables|Default|GetMaxPlayers)))
    (for _array_element_2 _connectedplayers
      (bind _aslobbyplayercontroller_2 (Class|BPILobbyPlayerController|LobbyPlayerControllerRef(Message) _array_element_2))
      (Default|AddPlayerInfo _aslobbyplayercontroller_2 (Variables|Default|GetConnectedPlayersInfo))
      (Default|UpdateAvailableCharacters _aslobbyplayercontroller_2 (Variables|Default|GetbAvailableCharacters))
      (CallFunction|AddtoKickList))
    (bind _array_element_3 (Utilities|Array|ForEachLoopwithBreak (Variables|Default|GetConnectedPlayersInfo))
      (:LoopBody
        (if (== (.PlayerCharacter (Utilities|Struct|BreakFPlayerInfo _array_element_3)) 0)
          (Variables|Default|SetbCanWeStart? false)
          (CallFunction|CannotStartGame)
          (else
            (Variables|Default|SetbCanWeStart? true)))))))

(event Custom|AddToKickList
  ;[1 1 1] Kick functionality
  ;;[1 1 1] AddToKickList - Add connected player to kick list.
  (bind _aslobbyplayercontroller (Class|BPILobbyPlayerController|LobbyPlayerControllerRef(Message) (Game|GetPlayerController 0)))
  (Default|AddPlayertoKickWindow _aslobbyplayercontroller))

(event Custom|CannotStartGame
  ;[1 1 1] Update all connected player's lobby widget information when called.
  (Utilities|Array|ForEachLoopwithBreak (Variables|Default|GetConnectedPlayersInfo)) ; enters at Break
)

(event Custom|LaunchGame
  ;[1 1 1] Shows loading screen and launches the game.
  (switch int (Variables|Default|GetMapID)
    (:0
      (Development|ExecuteConsoleCommand "servertravel /Game/Art/Maps/L_Debug_00" (Game|GetPlayerController 0)))
    (:1
      (Development|ExecuteConsoleCommand "servertravel /Game/Art/Maps/L_Debug_01" 0))))

(event Custom|ChangeCharacter
  (params (ConnectedPlayer :type Player%20Controller%20Object%20Reference) (CharacterClass :type Character%20Class%20Reference) (bChangedStatus? :type Boolean))
  (bind _returnvalue (Pawn|GetControlledPawn ConnectedPlayer))
  (bind _spawnpoints (Variables|Default|GetSpawnPoints))
  ;[1 1 1] ChangeCharacter - Spawn the selected character that the player chose in the Lobby.
  (if (not bChangedStatus?)
    (Utilities|IsValid _returnvalue
      (:Is%20Valid
        (Actor|DestroyActor _returnvalue))
      (:Is%20Not%20Valid
        _))
    (bind _returnvalue_2 (Game|SpawnActorfromClass CharacterClass (Transformation|GetActorTransform (Utilities|Array|Get(acopy) _spawnpoints (Math|Random|RandomIntegerinRange 0 (- (Utilities|Array|Length _spawnpoints) 1)))) "AdjustIfPossibleButAlwaysSpawn" ConnectedPlayer 0))
    (Pawn|Possess ConnectedPlayer _returnvalue_2)))

(event EventBeginPlay
  ;[1 1 1] BeginPlay
  (CallFunction|COut "BeginPlay" "Checking in." "(R=0.000000,G=1.000000,B=0.000000,A=1.000000)" false)
  ;[1 1 1] GetSet Server information.
  (bind _asbp_tiggameinstance (Class|BPIGameInstance|GameInstanceReference(Message) (Game|GetGameInstance)))
  (Variables|Default|SetAs%20BP%20Tig%20Game%20Instance _asbp_tiggameinstance)
  (Variables|Default|SetServerName (Variables|/Game/Core/GameInstances/BP_TigGameInstance.BP_TigGameInstance_C|GetServerName _asbp_tiggameinstance))
  (Variables|Default|SetMaxPlayers (Variables|/Game/Core/GameInstances/BP_TigGameInstance.BP_TigGameInstance_C|GetMaxPlayers _asbp_tiggameinstance)))

(event EventPostLogin
  (params (NewPlayer :type Player%20Controller%20Object%20Reference))
  ;[1 1 1] OnPostLogin - Initial setup that runs each time a player connects. The lobby must update for each connected player.
  (bind _output_get (Variables|Default|SetConnectedPlayer NewPlayer))
  (Utilities|Array|AddUnique (Variables|Default|GetConnectedPlayers) _output_get)
  (Utilities|FlowControl|Delay 1.0)
  (bind _aslobbyplayercontroller (Class|BPILobbyPlayerController|LobbyPlayerControllerRef(Message) (Variables|Default|GetConnectedPlayer)))
  (Default|InitialSetup _aslobbyplayercontroller (Variables|Default|GetServerName) (Variables|Default|GetSelectedMapImage) (Variables|Default|GetSelectedMapName) (Variables|Default|GetSelectedMapTime)))

(event EventOnLogout
  (params (ExitingController :type Controller%20Object%20Reference))
  (bind _connectedplayers (Variables|Default|GetConnectedPlayers))
  ;[1 1 1] Removes the connected player information and makes the character they were using avaiable to play as, then everyone updates with new info.
  (bind (_array_element _array_index) (Utilities|Array|ForEachLoopwithBreak _connectedplayers :!label _label)
    (:LoopBody
      (if (== _array_element ExitingController)
        (goto _label Break)))
    (:Completed
      (bind _aslobbyplayercontroller (Class|BPILobbyPlayerController|LobbyPlayerControllerRef(Message) (Utilities|Array|Get(acopy) _connectedplayers _array_index)))
      (Utilities|Array|SetArrayElem (Variables|Default|GetbAvailableCharacters) (Variables|/Game/Core/Controllers/PlayerControllers/BP_TigLobbyPlayerController.BP_TigLobbyPlayerController_C|GetSelectedCharacter _aslobbyplayercontroller) false)
      (Utilities|Array|RemoveIndex (Variables|Default|GetConnectedPlayers) _array_index)
      (Utilities|Array|RemoveIndex (Variables|Default|GetConnectedPlayersInfo) _array_index)
      (CallFunction|EveryoneUpdate))))

(fn ConstructionScript)

(fn GetSelectedCharacterIDClass
  (params (SelectedCharacterID :type Integer) (PreviousSelectionID :type Integer))
  (LocalVariables|SetLocal_SelectedCharacterID SelectedCharacterID)
  (LocalVariables|SetLocal_PreviousSelectionID PreviousSelectionID)
  (bind _asbp_tiggameinstance (Class|BPIGameInstance|GameInstanceReference(Message) (Game|GetGameInstance)))
  (LocalVariables|SetLocal_CharactersToSelect (Variables|/Game/Core/GameInstances/BP_TigGameInstance.BP_TigGameInstance_C|GetCharactersToSelect _asbp_tiggameinstance))
  (bind _asbp_tiglobbygamemode (Class|BPILobbyGameMode|LobbyGameModeReference(Message) (Game|GetGameMode)))
  (if (Utilities|Array|Get(acopy) (Variables|BP_TigLobbyGameMode_C|GetbAvailableCharacters _asbp_tiglobbygamemode) (LocalVariables|GetLocal_SelectedCharacterID))
    _
    (else
      (Utilities|Array|SetArrayElem (Variables|BP_TigLobbyGameMode_C|GetbAvailableCharacters _asbp_tiglobbygamemode) (LocalVariables|GetLocal_SelectedCharacterID) true)))
  (Utilities|Array|SetArrayElem (Variables|BP_TigLobbyGameMode_C|GetbAvailableCharacters _asbp_tiglobbygamemode) (LocalVariables|GetLocal_PreviousSelectionID) false)
  (return (Utilities|Array|Get(acopy) (LocalVariables|GetLocal_CharactersToSelect) (LocalVariables|GetLocal_SelectedCharacterID))))

(fn LobbyGameModeReference
  (return self))