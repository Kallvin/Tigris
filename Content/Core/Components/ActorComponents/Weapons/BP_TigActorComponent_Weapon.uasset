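; Actor component that handles weapon firing and ammo for its owner, dispatching by weapon type to a rifle or a telekinesis rifle.
; The rifle tracks a chambered round separately from the magazine, chambering from it when empty and playing an attached gunshot or dry-click sound.
; Reloading adds supplied ammo and chambers a round if needed, with helpers reporting magazine fullness and space.
; Telekinesis firing and both end-fire events are empty stubs.
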(event Custom|Fire
  (switch Utilities|FlowControl|Switch|SwitchonEWeaponType (Variables|Default|GetWeaponType)
    (:NewEnumerator1
      (CallFunction|FireRifle))
    (:NewEnumerator2
      (CallFunction|FireTelekinesisRifle))))

(event Custom|Reload%20Rifle
  (params (Ammo :type Integer%20%28by%20ref%29))
  ;[1 1 1] Reloading
  (Variables|Default|SetMagazine_Current (+ Ammo (Variables|Default|GetMagazine_Current)))
  (if (> (Variables|Default|GetChamber) 0) ; Don't rack chamber?
    _
    (else
      (Math|Integer|DecrementInt (Variables|Default|GetMagazine_Current)
        (:%20%20
          (Math|Integer|IncrementInt (Variables|Default|GetChamber)
            (:%20%20
              _))))))
  (CallFunction|COut "Reload Rifle" "Reloaded" "(R=0.000000,G=1.000000,B=1.000000,A=1.000000)" false))

(event Custom|Fire%20Telekinesis%20Rifle)

(event Custom|End%20Telekinesis%20Rifle)

(event Custom|End%20Fire%20Rifle)

(fn MagazineIsFull
  (return (== (Variables|Default|GetMagazine_Current) (Variables|Default|GetMagazine_Max))))

(fn AmmoNeeded
  (return (Math|Integer|Clamp(Integer) (- (Variables|Default|GetMagazine_Max) (Variables|Default|GetMagazine_Current)) 0 (Variables|Default|GetMagazine_Max))))

(fn FireRifle
  (if (> (Variables|Default|GetChamber) 0) ; Round In chamber check.
    _
    (else
      ;[1 1 1] Cycle for ammo - Or not.
      (if (> (Variables|Default|GetMagazine_Current) 0) ; Out of ammo check.
        (Math|Integer|DecrementInt (Variables|Default|GetMagazine_Current)
          (:%20%20
            (Math|Integer|IncrementInt (Variables|Default|GetChamber)
              (:%20%20
                _))))
        (else
          (Audio|SpawnSoundAttached "/Game/Art/Sounds/WaveFiles/Lights/A_LightSwitch_04_01.A_LightSwitch_04_01" (Variables|/Script/Engine.Actor|GetRootComponent (Components|GetOwner)) "Weapon" "0, 0, 0" "0, 0, 0" "KeepRelativeOffset" false 1.0 1.0 0.0 "/Game/Art/Sounds/Attenuations/Character/ATT_FootstepsSound.ATT_FootstepsSound" 0)
          (return false)))))
  (Math|Integer|DecrementInt (Variables|Default|GetChamber) ; Let loose the lead!
    (:%20%20
      ;[1 1 1] Fire
      (Audio|SpawnSoundAttached "/Game/Art/Sounds/WaveFiles/Weapons/Rifle/A_Gun_00.A_Gun_00" (Variables|/Script/Engine.Actor|GetRootComponent (Components|GetOwner)) "Weapon" "0, 0, 0" "0, 0, 0" "KeepRelativeOffset" false 1.0 1.0 0.0 "/Game/Art/Sounds/Attenuations/Character/ATT_FootstepsSound.ATT_FootstepsSound" 0)
      (return true))))