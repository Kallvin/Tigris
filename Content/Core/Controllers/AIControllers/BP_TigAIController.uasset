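; BP_TigAIController is an AI controller that makes its controlled pawn wander at random.
; On BeginPlay it logs a check-in message and starts a looping timer on Update, with a randomized initial delay, storing the handle.
; Each Update sends the pawn via AI MoveTo to a random reachable point around its current location.
; Rotation-interpolation nodes are left unconnected, so no custom turning runs.
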(event Custom|Update
  (bind _returnvalue (Pawn|GetControlledPawn))
  ;[1 1 1] Update Timer
  (AI|AIMoveTo _returnvalue (.RandomLocation (AI|Navigation|GetRandomReachablePointinRadius (Transformation|GetActorLocation _returnvalue) 1e+03 0 0)) 0 5.0 false))

(event EventBeginPlay
  ;[1 1 1] Begin Play
  (CallFunction|COut "BeginPlay" "Checking in." "(R=0.000000,G=1.000000,B=0.000000,A=1.000000)" false)
  (bind _returnvalue (Utilities|Time|SetTimerbyFunctionName self "Update" 1e+01 true 3.0 2.0))
  (Variables|Default|SetUpdateTimerHandle _returnvalue))

(fn ConstructionScript)