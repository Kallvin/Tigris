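; BP_TigPlayerController is the player controller that handles debug hotkeys, quitting and mouse cursor toggling.
; A FlipFlop on ToggleMouseInputMode drives MouseCursorVisibilty, which sets cursor display and click events together.
; Debug inputs toggle the BP_TigHUD info panel, damage the controlled pawn, flip log and screen printing on BP_TigGameInstance, or disable on-screen messages.
; Status and failed casts are reported through COut.
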(event Custom|MouseCursorVisibilty
  (params (bNewVisibiltyRequest :type Boolean))
  ;[1 1 1] UI
  (Variables|Default|SetbShowMouseCursor bNewVisibiltyRequest)
  (Variables|Default|SetbEnableClickEvents bNewVisibiltyRequest))

(event EventBeginPlay
  (CallFunction|COut "BeginPlay" "Checking in." "(R=0.000000,G=1.000000,B=0.000000,A=1.000000)" false))

(event Input|ActionEvents|InputActionQuit
  (params (Key :type Key%20Structure :default "None"))
  ;[1 1 1] Debug
  (:Pressed
    (Game|QuitGame 0 "Quit" false)))

(event Input|ActionEvents|InputActionToggleDebugInfo
  (params (Key :type Key%20Structure :default "None"))
  (bind _returnvalue (HUD|GetHUD))
  ;[1 1 1] Debug
  (:Pressed
    (Utilities|IsValid _returnvalue
      (:Is%20Valid
        (bind _asbp_tig_hud (Utilities|Casting|CastToBP_TigHUD _returnvalue)
          (:then
            (Default|ToggleDebugInfoPanelVisibility (Variables|/Game/Core/HUDs/BP_TigHUD.BP_TigHUD_C|GetWBP_HUD_Elements _asbp_tig_hud)))
          (:CastFailed
            (CallFunction|COut "ToggleDebugInfo" "BP_TigHUD" "(R=0.000000,G=1.000000,B=1.000000,A=1.000000)" true)))))))

(event Input|ActionEvents|InputActionDebugDamage
  (params (Key :type Key%20Structure :default "None"))
  (bind _returnvalue (Pawn|GetControlledPawn))
  ;[1 1 1] Debug
  ;;[1 1 1] DebugDamage
  (:Pressed
    (Utilities|IsValid _returnvalue
      (:Is%20Valid
        (bind _returnvalue_2 (Game|Damage|ApplyDamage _returnvalue 1.0 0 _returnvalue))
        (CallFunction|COut "DebugDamage" (Utilities|Text|FormatText "Dmg: {Dmg} Stop hitting yourself!" _returnvalue_2) "(R=0.000000,G=1.000000,B=1.000000,A=1.000000)" false)))))

(event Input|ActionEvents|InputActionToggleDebugPrintToLog
  (params (Key :type Key%20Structure :default "None"))
  ;[1 1 1] Debug
  ;;[1 1 1] DebugPrintToggles
  (:Pressed
    (bind _asbp_tig_game_instance (Utilities|Casting|CastToBP_TigGameInstance (Game|GetGameInstance))
      (:then
        (Default|ToggleDebugPrinttoLog _asbp_tig_game_instance))
      (:CastFailed
        (CallFunction|COut "ToggleDebugPrintToLog" "BP_TigGameInstance" "(R=0.000000,G=1.000000,B=1.000000,A=1.000000)" true)))))

(event Input|ActionEvents|InputActionToggleDebugPrintToScreen
  (params (Key :type Key%20Structure :default "None"))
  ;[1 1 1] Debug
  ;;[1 1 1] DebugPrintToggles
  (:Pressed
    (bind _asbp_tig_game_instance (Utilities|Casting|CastToBP_TigGameInstance (Game|GetGameInstance))
      (:then
        (Default|ToggleDebugPrinttoScreen _asbp_tig_game_instance))
      (:CastFailed
        (CallFunction|COut "ToggleDebugPrintToScreen" "BP_TigGameInstance" "(R=0.000000,G=1.000000,B=1.000000,A=1.000000)" true)))))

(event Input|ActionEvents|InputActionDisableAllOnScreenMessages
  (params (Key :type Key%20Structure :default "None"))
  ;[1 1 1] Debug
  ;;[1 1 1] DebugPrintToggles
  (:Pressed
    (Development|ExecuteConsoleCommand "DisableAllScreenMessages" 0)))

(event Input|ActionEvents|InputActionToggleMouseInputMode
  (params (Key :type Key%20Structure :default "None"))
  ;[1 1 1] Input
  (:Pressed
    (bind _isa (Utilities|FlowControl|FlipFlop)
      (:A
        _)
      (:B
        _))
    (CallFunction|MouseCursorVisibilty _isa)))

(fn ConstructionScript)