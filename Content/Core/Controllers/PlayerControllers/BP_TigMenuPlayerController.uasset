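; BP_TigMenuPlayerController is the player controller for the main menu.
; One second after BeginPlay it enables the mouse cursor and click events, then asks the game instance to show the main menu message.
; The Quit input action exits the game.
; Helper functions cache the Tig HUD and menu game mode with logging on failed casts, though nothing in this file calls them.
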(event Custom|MouseCursorVisibiltyAndClickEvents
  (params (bNewVisibiltyRequest :type Boolean))
  ;[1 1 1] UI
  (Variables|Default|SetbShowMouseCursor bNewVisibiltyRequest)
  (Variables|Default|SetbEnableClickEvents bNewVisibiltyRequest))

(event EventBeginPlay
  (CallFunction|COut "BeginPlay" "Checking in." "(R=0.000000,G=1.000000,B=0.000000,A=1.000000)" false)
  (Utilities|FlowControl|Delay 1.0)
  (CallFunction|MouseCursorVisibiltyandClickEvents self true)
  (Class|BPIGameInstance|ShowMainMenu(Message) (Game|GetGameInstance)))

(event Input|ActionEvents|InputActionQuit
  (params (Key :type Key%20Structure :default "None"))
  ;[1 1 1] Debug
  (:Pressed
    (Game|QuitGame 0 "Quit" false)))

(fn ConstructionScript)

(fn GetSetHUD
  (bind _asbp_tig_hud (Utilities|Casting|CastToBP_TigHUD (HUD|GetHUD))
    (:then
      (Variables|HUD|SetAs%20BP%20Tig%20HUD _asbp_tig_hud))
    (:CastFailed
      (CallFunction|COut "BeginPlay" "BP_TigHUD" "(R=0.000000,G=1.000000,B=0.000000,A=1.000000)" true)))
  (return))

(fn GetSetGameMode
  (bind _asbp_tig_menu_game_mode (Utilities|Casting|CastToBP_TigMenuGameMode (Game|GetGameMode))
    (:then
      (Variables|Default|SetAs%20BP%20Tig%20Menu%20Game%20Mode _asbp_tig_menu_game_mode))
    (:CastFailed
      (CallFunction|COut "BeginPlay" "BP_TigGameMode" "(R=0.000000,G=1.000000,B=0.000000,A=1.000000)" true)))
  (return))