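; Player controller for the multiplayer lobby, linking each player's lobby widget to the lobby game mode and game instance.
; It creates the menu and updates its map info, player list, available characters and chat.
; Character picks and chat go through the game mode, reached by interface messages, to update all players.
; It also toggles lobby visibility, shows loading and error widgets, and destroys the session on kick or EndPlay.
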(event Custom|MouseCursorVisibiltyAndClickEvents
  (params (bNewVisibiltyRequest :type Boolean))
  ;[1 1 1] Kal's chopping block. Questionable at best functionality.
  ;;[1 1 1] UI
  (Variables|Default|SetbShowMouseCursor bNewVisibiltyRequest)
  (Variables|Default|SetbEnableClickEvents bNewVisibiltyRequest))

(event Custom|InitialSetup
  (params (ServerName :type Text) (MapImage :type Texture%202D%20Object%20Reference) (MapName :type Text) (MapTime :type Text))
  ;[1 1 1] InitialSetup - Tells server to update.
  (CallFunction|SetupLobbyMenu ServerName)
  (Utilities|FlowControl|Delay 0.1)
  (CallFunction|UpdateLobbySettings MapImage MapName MapTime)
  (Default|SaveGame (Variables|Default|GetAs%20BP%20Tig%20Game%20Instance)) ; Necessary on InitialSetup? Up for debate but it seems to cause an issue with initial players being treated as an existing player.
)

(event Custom|UpdateNumberOfPlayers
  (params (CurrentPlayers :type Integer%20%28by%20ref%29) (MaxPlayers :type Integer%20%28by%20ref%29))
  ;[1 1 1] UpdateNumberOfPlayers - Update and display the number of current connected players.
  (Default|UpdatePlayersDisplay (Variables|Default|GetLobbyWidget) (Utilities|Text|FormatText "{Current} of {Max}" CurrentPlayers MaxPlayers)))

(event Custom|AddPlayerInfo
  (params (PlayersInfo :type Array%20of%20F%20Player%20Info%20Structures))
  ;[1 1 1] AddPlayerInfo - Updates the player list window in the WBP_LobbyMenu.
  (Variables|Default|SetAllConnectedPlayers PlayersInfo)
  (bind _lobbywidget (Variables|Default|GetLobbyWidget)
    (:then
      (Default|ClearPlayerList _lobbywidget)
      (for _array_element (Variables|Default|GetAllConnectedPlayers)
        (Default|UpdatePlayerWindow (Variables|Default|GetLobbyWidget) _array_element)))
    (:else)))

(event Custom|UpdateAvailableCharacters
  (params (bAvailableCharacters :type Array%20of%20Booleans))
  ;[1 1 1] UpdateAvailableCharacters - Update to client which characters are available
  (Variables|Default|SetAvailable%20Characters bAvailableCharacters)
  (bind _lobbywidget (Variables|Default|GetLobbyWidget)
    (:then
      (Default|UpdateCharactersAvailable _lobbywidget (Variables|Default|GetAvailable%20Characters)))
    (:else)))

(event Custom|AddPlayerToKickWindow
  ;[1 1 1] AddPlayerToKickWindow - Adds the player to the window to be kicked.
  (bind _lobbywidget (Variables|Default|GetLobbyWidget)
    (:then
      (Default|AddPlayertoKickWindow _lobbywidget))
    (:else)))

(event Custom|GetChatMessage
  (params (TextToSend :type Text))
  ;[1 1 1] GetChatMessage - Get incoming chat message and tell all players to update their chat window.
  (Variables|Default|SetSenderText TextToSend)
  (Variables|Default|SetSenderName (.Name (Utilities|Struct|BreakFPlayerInfo (Variables|/Game/Core/GameInstances/BP_TigGameInstance.BP_TigGameInstance_C|GetPlayers%20Info (Variables|Default|GetAs%20BP%20Tig%20Game%20Instance)))))
  (bind _asbp_tiglobbygamemode (Class|BPILobbyGameMode|LobbyGameModeReference(Message) (Game|GetGameMode)))
  (for _array_element (Variables|/Game/Core/GameModes/BP_TigLobbyGameMode.BP_TigLobbyGameMode_C|GetConnectedPlayers _asbp_tiglobbygamemode)
    (bind _aslobbyplayercontroller (Class|BPILobbyPlayerController|LobbyPlayerControllerRef(Message) _array_element))
    (CallFunction|UpdateChat _aslobbyplayercontroller (Variables|Default|GetSenderName) (Variables|Default|GetSenderText))))

(event Custom|UpdateChat
  (params (SenderName :type Text) (SenderText :type Text))
  ;[1 1 1] UpdateChat - Updates the chat window in the lobby widget menu.
  (Default|UpdateChat (Variables|Default|GetLobbyWidget) SenderName SenderText))

(event Custom|SetupLobbyMenu
  (params (ServerName :type Text))
  ;[1 1 1] SetupLobbyMenu - Setup and display the lobby menu to each connected player.
  (Variables|Default|SetbShowMouseCursor true)
  (bind _returnvalue (UserInterface|CreateWidget "/Game/Core/Widgets/Menu/WBP_LobbyMenu.WBP_LobbyMenu_C" self ServerName))
  (bind _output_get (Variables|Default|SetLobbyWidget _returnvalue))
  (UserInterface|Viewport|AddtoViewport _output_get 0)
  (Input|SetInputModeGameandUI self (Variables|Default|GetLobbyWidget) "DoNotLock" true))

(event Custom|UpdateLobbySettings
  (params (MapImage :type Texture%202D%20Object%20Reference%20%28by%20ref%29) (MapName :type Text%20%28by%20ref%29) (MapTime :type Text%20%28by%20ref%29))
  ;[1 1 1] UpdateLobbySettings - Update the lobby information on client.
  (Default|UpdateLobbyInfo (Variables|Default|GetLobbyWidget) MapImage MapName MapTime))

(event Custom|CallUpdate
  (params (PlayerInfo :type F%20Player%20Info%20Structure) (bChangedStatus? :type Boolean))
  ;[1 1 1] Call Update - Assigns the updated selected character and tells everyone on the server to update their lobby window.
  (bind _asbp_tiglobbygamemode (Class|BPILobbyGameMode|LobbyGameModeReference(Message) (Game|GetGameMode)))
  (Default|ChangeCharacter _asbp_tiglobbygamemode self (.PlayerCharacter (Utilities|Struct|BreakFPlayerInfo PlayerInfo)) bChangedStatus?)
  (Default|EveryoneUpdate _asbp_tiglobbygamemode))

(event Custom|ShowLoadingScreen
  ;[1 1 1] ShowLoadingScreen - Removes the lobby widget and displays the loading screen while level loads in the background.
  (Widget|RemovefromParent (Variables|Default|GetLobbyWidget))
  (bind _returnvalue (UserInterface|CreateWidget "/Game/Core/Widgets/Menu/WBP_LoadingScreen.WBP_LoadingScreen_C" self))
  (UserInterface|Viewport|AddtoViewport _returnvalue 0))

(event Custom|Kicked
  ;[1 1 1] Kicked & EndPlay - Called when the server disconnects or player is kicked.
  (Game|OpenLevel(byObjectReference) "/Game/Art/Maps/L_Main.L_Main")
  (|DestroySession self))

(event Custom|AssignSelectedCharacter
  (params (SelectedCharacter :type Integer) (CharacterImage :type Texture%202D%20Object%20Reference))
  ;[1 1 1] AssignSelectedCharacter - Handle character selection and determine if the selected character is available to be assigned.
  (Variables|Default|SetPrevious%20Selection (Variables|Default|GetSelectedCharacter))
  (Variables|Default|SetSelectedCharacter SelectedCharacter)
  (Variables|Default|SetCharacterImage CharacterImage)
  (bind _asbp_tiglobbygamemode (Class|BPILobbyGameMode|LobbyGameModeReference(Message) (Game|GetGameMode)))
  (bind _character (Default|GetSelectedCharacterIDClass _asbp_tiglobbygamemode (Variables|Default|GetSelectedCharacter) (Variables|Default|GetPrevious%20Selection)))
  (CallFunction|AssignPlayer (Variables|Default|GetCharacterImage) _character))

(event Custom|AssignPlayer
  (params (PlayerImage :type Texture%202D%20Object%20Reference) (PlayerCharacter :type Character%20Class%20Reference))
  ;[1 1 1] AssignPlayer - Assigns the selected character and tells everyone to update.
  (bind _structout (Utilities|Struct|SetmembersinFPlayerInfo (Variables|/Game/Core/GameInstances/BP_TigGameInstance.BP_TigGameInstance_C|GetPlayers%20Info (Variables|Default|GetAs%20BP%20Tig%20Game%20Instance)) PlayerImage PlayerCharacter))
  (Default|SaveGame (Variables|Default|GetAs%20BP%20Tig%20Game%20Instance))
  (CallFunction|CallUpdate _structout false) ; Supposedly configurable to take an input of character class. This is in reference to the SaveGame to the left of this node.
)

(event EventBeginPlay
  ;[1 1 1] BeginPlay
  (CallFunction|COut "BeginPlay" "Checking in." "(R=0.000000,G=1.000000,B=0.000000,A=1.000000)" false)
  (bind _asbp_tiggameinstance (Class|BPIGameInstance|CustomGameInstanceRef(Message) (Game|GetGameInstance)))
  (Variables|Default|SetAs%20BP%20Tig%20Game%20Instance _asbp_tiggameinstance))

(event EventEndPlay
  (params (EndPlayReason :type EEndPlayReason%20Enum :default "Destroyed"))
  ;[1 1 1] Kicked & EndPlay - Called when the server disconnects or player is kicked.
  (|DestroySession self))

(event Input|ActionEvents|InputActionQuit
  (params (Key :type Key%20Structure))
  ;[1 1 1] Kal's chopping block. Questionable at best functionality.
  ;;[1 1 1] Debug
  (:Pressed
    (Game|QuitGame 0 "Quit" false)))

(event Input|KeyboardEvents|T
  (params (Key :type Key%20Structure))
  (bind _self self)
  (bind _lobbywidget (Variables|Default|GetLobbyWidget))
  ;[1 1 1] InputAction T - Hide Lobby Window.
  (:Pressed
    (Utilities|FlowControl|FlipFlop
      (:A
        (Widget|SetVisibility _lobbywidget "Hidden")
        (Variables|Default|SetbShowMouseCursor false)
        (Input|SetInputModeGameOnly _self))
      (:B
        (Widget|SetVisibility _lobbywidget "Visible")
        (Variables|Default|SetbShowMouseCursor true)
        (Input|SetInputModeGameandUI _self 0 "DoNotLock" true)))))

(fn ConstructionScript)

(fn CreateErrorMessage
  (params (ErrorMessage :type Text))
  (bind _errorwindow (Variables|Default|GetErrorWindow)
    (:then
      (if (UserInterface|Viewport|IsinViewport _errorwindow)
        (Widget|RemovefromParent _errorwindow)
        (bind _returnvalue (UserInterface|CreateWidget "/Game/Core/Widgets/Menu/WBP_ErrorWindow.WBP_ErrorWindow_C" self :!label _label))
        (bind _output_get (Variables|Default|SetErrorWindow _returnvalue))
        (UserInterface|Viewport|AddtoViewport _output_get 1)))
    (:else
      (goto _label)))
  (Default|SetMessage (.AsWBP%20Error%20Window (Utilities|Casting|CastToWBP_ErrorWindow (Variables|Default|GetErrorWindow))) ErrorMessage)
  (return))

(fn LobbyPlayerControllerRef
  (return self))