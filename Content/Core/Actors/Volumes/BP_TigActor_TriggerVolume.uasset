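; BP_TigActor_TriggerVolume is a paired teleporter that moves the player character to its PartnerTriggerVolume's raised location and rotation.
; Box overlap outside cooldown calls the teleport function, which cools down the partner before moving the player, preventing an immediate bounce back.
; Both cooldowns start even for non-player overlaps, since the class check only gates the move.
; A timeline times each cooldown, turning the indicator mesh red and animating its color until finished.
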(event OnComponentBeginOverlap(Box)
  (params (OverlappedComponent :type Primitive%20Component%20Object%20Reference) (OtherActor :type Actor%20Object%20Reference) (OtherComp :type Primitive%20Component%20Object%20Reference) (OtherBodyIndex :type Integer) (bFromSweep :type Boolean) (SweepResult :type Hit%20Result%20Structure%20%28by%20ref%29))
  ;[1 1 1] Trigger function
  (if (Variables|Default|GetbOnCooldown?)
    (CallFunction|COut "OnComponentBeginOverlap(Box)" "Teleporter is  cooling down. bOnCooldown? = true." "(R=0.000000,G=1.000000,B=1.000000,A=1.000000)" false)
    (else
      (CallFunction|TeleportPlayertoPartnerTriggerVolume OtherActor)
      (CallFunction|IndicatorCooldown))))

(event Custom|SetColor
  (params (NewColor :type Linear%20Color%20Structure :default "(R=1.000000,G=0.000000,B=0.000000,A=1.000000)"))
  (Rendering|Material|SetVectorParameterValueonMaterials (Variables|Default|GetStaticMesh_Indicator) "Base Color" (Math|Conversions|ToVector(LinearColor) NewColor)))

(event Custom|IndicatorCooldown
  (Variables|Default|SetbOnCooldown? true)
  (CallFunction|SetColor "(R=1.000000,G=0.000000,B=0.000000,A=1.000000)")
  (bind _indicatorcolor (Timeline|Indicator PlayFromStart)
    (:Update
      (Rendering|Material|SetVectorParameterValueonMaterials (Variables|Default|GetStaticMesh_Indicator) "Base Color" _indicatorcolor))
    (:Finished
      (Variables|Default|SetbOnCooldown? false))))

(event EventBeginPlay
  (|CallParentFunction)
  (CallFunction|COut "BeginPlay" "Checking in." "(R=0.000000,G=1.000000,B=0.000000,A=1.000000)" false))

(fn ConstructionScript
  (|CallParentFunction))

(fn CheckforPlayer
  (params (Object :type Object%20Object%20Reference))
  (return (== (Utilities|GetClass Object) "/Game/Core/Actors/Pawns/Characters/PlayerCharacters/BP_TigCharacter_Player.BP_TigCharacter_Player_C")))

(fn TeleportPlayertoPartnerTriggerVolume
  (params (OtherActor :type Actor%20Object%20Reference))
  (bind _partner_triggervolume (Variables|References|GetPartner_TriggerVolume))
  (bind _returnvalue (Transformation|GetActorTransform _partner_triggervolume))
  (Utilities|IsValid (Variables|References|GetPartner_TriggerVolume)
    (:Is%20Valid
      (CallFunction|IndicatorCooldown (Variables|References|GetPartner_TriggerVolume))
      (if (References|CheckforPlayer OtherActor)
        (Transformation|SetActorLocationAndRotation OtherActor (+ (.location _returnvalue) "0, 0,92.000000") (.rotation _returnvalue) false true)
        (CallFunction|COut "OnActorBeginOverlap" "Teleporting player character." "(R=0.000000,G=1.000000,B=1.000000,A=1.000000)" false)))))