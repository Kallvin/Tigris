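; BP_TigActor_Volume_KillZ is a kill volume that triggers death for player characters entering it.
; The construction script sizes its box from Bounds, and begin overlap passes the other actor to HandleOverlapKillZ.
; That function calls Death on BP_TigCharacter_Player; for other valid actors, DestroyActor has no target, so it destroys the volume itself despite logging the other actor.
; COut logs startup, kills and invalid actors.
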(event OnComponentBeginOverlap(Box_Volume_KillZ)
  (params (OverlappedComponent :type Primitive%20Component%20Object%20Reference) (OtherActor :type Actor%20Object%20Reference) (OtherComp :type Primitive%20Component%20Object%20Reference) (OtherBodyIndex :type Integer) (bFromSweep :type Boolean) (SweepResult :type Hit%20Result%20Structure%20%28by%20ref%29))
  (CallFunction|HandleOverlapKillZ OtherActor))

(event EventBeginPlay
  (|CallParentFunction)
  (CallFunction|COut "BeginPlay" "Checking in." "(R=0.000000,G=1.000000,B=0.000000,A=1.000000)" false))

(fn ConstructionScript
  (|CallParentFunction)
  (Components|Box|SetBoxExtent (Variables|Default|GetBox_Volume_KillZ) (Variables|Default|GetBounds) true))

(fn HandleOverlapKillZ
  (params (Actor :type Actor%20Object%20Reference))
  (bind _output_get (LocalVariables|SetLocal_Actor Actor))
  (Utilities|IsValid _output_get
    (:Is%20Valid
      (CallFunction|COut "OnComponentBeginOverlap(Box_Volume_KillZ)" (Utilities|Text|FormatText "Destroying {Actor}" (LocalVariables|GetLocal_Actor)) "(R=1.000000,G=1.000000,B=0.000000,A=1.000000)" false)
      (bind _asbp_tig_character_player (Utilities|Casting|CastToBP_TigCharacter_Player (LocalVariables|GetLocal_Actor))
        (:then
          (Default|Death _asbp_tig_character_player))
        (:CastFailed
          (Actor|DestroyActor)))
      (return))
    (:Is%20Not%20Valid
      (CallFunction|COut "HandleOverlapKillZ" "Actor is no longer valid while trying to destroy or mark it for death." "(R=0.000000,G=1.000000,B=1.000000,A=1.000000)" false))))