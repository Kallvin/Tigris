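; BP_TigActor_Interactables_Button is an interactable button actor that plays a click sound when pressed.
; The button mesh's OnClicked event and the Interact event share one path, which logs through COut and plays the sound at the mesh's world location.
; BeginPlay and the construction script call their parent versions, with BeginPlay also logging a check-in.
; No other press behavior is wired here.
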(event OnClicked(StaticMesh_Button)
  (params (TouchedComponent :type Primitive%20Component%20Object%20Reference) (ButtonPressed :type Key%20Structure :default "None"))
  (CallFunction|COut "BeginPlay" "Click." "(R=0.000000,G=1.000000,B=1.000000,A=1.000000)" false)
  (Audio|PlaySoundatLocation "/Engine/VREditor/Sounds/UI/Click_on_Button.Click_on_Button" (Transformation|GetWorldLocation (Variables|Default|GetStaticMesh_Button)) "0, 0, 0" 1.0 1.0 0.0 0 0 self))

(event EventBeginPlay
  (|CallParentFunction)
  (CallFunction|COut "BeginPlay" "Checking in." "(R=0.000000,G=1.000000,B=0.000000,A=1.000000)" false))

(event EventInteract
  (params (Interactor :type Object%20Object%20Reference%20%28by%20ref%29))
  (CallFunction|COut "BeginPlay" "Click." "(R=0.000000,G=1.000000,B=1.000000,A=1.000000)" false)
  (Audio|PlaySoundatLocation "/Engine/VREditor/Sounds/UI/Click_on_Button.Click_on_Button" (Transformation|GetWorldLocation (Variables|Default|GetStaticMesh_Button)) "0, 0, 0" 1.0 1.0 0.0 0 0 self))

(fn ConstructionScript
  (|CallParentFunction))