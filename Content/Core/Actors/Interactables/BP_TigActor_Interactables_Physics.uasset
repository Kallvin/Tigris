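; Physics interactable actor that plays an impact sound when its static mesh takes a hard enough hit.
; Hits whose normal impulse exceeds MinimumImpulseOnHit spawn A_Ball_Cue attached to the mesh at the impact location, using footstep attenuation and ball concurrency settings.
; ImpactSoundType feeds the cue's Floor parameter to select the sound, with IsMale always set to true.
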(event OnComponentHit(StaticMesh)
  (params (HitComponent :type Primitive%20Component%20Object%20Reference) (OtherActor :type Actor%20Object%20Reference) (OtherComp :type Primitive%20Component%20Object%20Reference) (NormalImpulse :type Vector :default "0, 0, 0") (Hit :type Hit%20Result%20Structure%20%28by%20ref%29))
  (if (> (Math|Vector|VectorLength NormalImpulse) (Variables|Default|GetMinimumImpulseOnHit))
    (bind _returnvalue (Audio|SpawnSoundAttached "/Game/Art/Sounds/SoundCues/Basic/A_Ball_Cue.A_Ball_Cue" (Variables|Default|GetStaticMesh) "None" (.Location (Collision|BreakHitResult Hit)) "0, 0, 0" "KeepWorldPosition" true 1.0 1.0 0.0 "/Game/Art/Sounds/Attenuations/Character/ATT_FootstepsSound.ATT_FootstepsSound" "/Game/Art/Sounds/ConcurrencySettings/Ball_SC.Ball_SC"))
    (Effects|Components|ParticleSystem|SetBoolParameter _returnvalue "IsMale" true)
    (Effects|Components|ParticleSystem|SetIntParameter _returnvalue "Floor" (Variables|Default|GetImpactSoundType))))

(event EventBeginPlay
  (|CallParentFunction))

(fn ConstructionScript
  (|CallParentFunction))