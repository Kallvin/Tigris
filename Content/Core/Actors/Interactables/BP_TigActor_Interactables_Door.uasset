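; Interactable door actor that the player character opens and closes through Interact unless it is locked.
; Multicast events play or reverse one timeline that swings the mesh's yaw with sweep, setting IsOpen from an angle threshold.
; With auto-close enabled, the door closes when the player leaves its box.
; The construction script applies an optional material, and clicking the mesh plays a sound.
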(event OnClicked(StaticMesh_Door)
  (params (TouchedComponent :type Primitive%20Component%20Object%20Reference) (ButtonPressed :type Key%20Structure :default "None"))
  (CallFunction|COut "BeginPlay" "Click." "(R=0.000000,G=1.000000,B=1.000000,A=1.000000)" false)
  (Audio|PlaySoundatLocation "/Engine/VREditor/Sounds/UI/Click_on_Button.Click_on_Button" (Transformation|GetWorldLocation (Variables|Default|GetStaticMesh_Door)) "0, 0, 0" 1.0 1.0 0.0 0 0 self))

(event OnComponentEndOverlap(Box)
  (params (OverlappedComponent :type Primitive%20Component%20Object%20Reference) (OtherActor :type Actor%20Object%20Reference) (OtherComp :type Primitive%20Component%20Object%20Reference) (OtherBodyIndex :type Integer))
  (if (Variables|Overlap|GetbAutoCloseDoor?)
    (if (== (Utilities|GetClass OtherActor) "/Game/Core/Actors/Pawns/Characters/PlayerCharacters/BP_TigCharacter_Player.BP_TigCharacter_Player_C")
      (CallFunction|MultiCloseDoor))))

(event Custom|Multi_OpenDoor
  (bind _staticmesh_door (Variables|Default|GetStaticMesh_Door))
  (bind _returnvalue (Transformation|GetRelativeTransform _staticmesh_door))
  ;[1 1 1] MultiCast - Open and close door timeline sets the rotation to the desired position.
  (bind _doorposition (Timeline|Open_Door Play)
    (:Update
      (Transformation|SetRelativeRotation (Variables|Default|GetStaticMesh_Door) (Math|Rotator|MakeRotator (.roll (.rotation _returnvalue)) (.pitch (.rotation _returnvalue)) _doorposition) true false)
      (Math|Float|CompareFloat _doorposition 7e+01
        (:>
          (Variables|Default|SetbIsOpen? true))
        (:==
          (Variables|Default|SetbIsOpen? false :!label _label))
        (:<
          (goto _label))))))

(event Custom|Multi_CloseDoor
  (bind _staticmesh_door (Variables|Default|GetStaticMesh_Door))
  (bind _returnvalue (Transformation|GetRelativeTransform _staticmesh_door))
  ;[1 1 1] MultiCast - Open and close door timeline sets the rotation to the desired position.
  (bind _doorposition (Timeline|Open_Door Reverse)
    (:Update
      (Transformation|SetRelativeRotation (Variables|Default|GetStaticMesh_Door) (Math|Rotator|MakeRotator (.roll (.rotation _returnvalue)) (.pitch (.rotation _returnvalue)) _doorposition) true false)
      (Math|Float|CompareFloat _doorposition 7e+01
        (:>
          (Variables|Default|SetbIsOpen? true))
        (:==
          (Variables|Default|SetbIsOpen? false :!label _label))
        (:<
          (goto _label))))))

(event EventBeginPlay
  (|CallParentFunction)
  (CallFunction|COut "BeginPlay" "Checking in." "(R=0.000000,G=1.000000,B=0.000000,A=1.000000)" false))

(event EventInteract
  (params (Interactor :type Object%20Object%20Reference%20%28by%20ref%29))
  (if (not (Variables|Access|GetbIsLocked?))
    (if (== (Utilities|GetClass Interactor) "/Game/Core/Actors/Pawns/Characters/PlayerCharacters/BP_TigCharacter_Player.BP_TigCharacter_Player_C")
      (if (Variables|Default|GetbIsOpen?)
        (CallFunction|MultiCloseDoor)
        (else
          (CallFunction|MultiOpenDoor))))))

(fn ConstructionScript
  (|CallParentFunction)
  (if (not (== (Variables|Default|GetMaterialInstance_Door) 0))
    (Rendering|Material|SetMaterial (Variables|Default|GetStaticMesh_Door) 0 (Variables|Default|GetMaterialInstance_Door))))