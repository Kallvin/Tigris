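; Prototype projectile actor meant to penetrate surfaces on bounce, teleporting to an exit point at half velocity or being destroyed.
; A looping timer and the bounce handler draw debug trail lines, colored by current-to-initial speed ratio.
; Exit search sphere-traces backward from beyond the impact along its velocity.
; Penetration is unfinished: the threshold check has no effect, the trace result never reaches a return, and the energy-based speed function is uncalled.
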(event OnProjectileBounce(ProjectileMovement)
  (params (ImpactResult :type Hit%20Result%20Structure%20%28by%20ref%29) (ImpactVelocity :type Vector%20%28by%20ref%29 :default "0, 0, 0"))
  (bind _location (Collision|BreakHitResult ImpactResult))
  (Rendering|Debug|DrawDebugLine (Variables|Default|GetLastPosition) _location (CallFunction|GetTraceColor) (Variables|Default|GetTraceDuration) 0.0)
  (Variables|Default|SetLastPosition _location)
  ;[1 1 1] Determine penetrate
  (CallFunction|DeterminePenetration ImpactVelocity)
  ;[1 1 1] Find Exit Location
  (bind (_exitlocation _bresultfound_) (CallFunction|ComputeExitLocation ImpactVelocity ImpactResult))
  (if _bresultfound_
    (Transformation|SetActorTransform (Math|Transform|MakeTransform _exitlocation) false true)
    (Variables|/Script/Engine.MovementComponent|SetVelocity (Variables|Default|GetProjectileMovement) (* (Variables|/Script/Engine.MovementComponent|GetVelocity (Variables|Default|GetProjectileMovement)) 0.5))
    (else
      (Actor|DestroyActor))))

(event Custom|Update
  (bind _returnvalue (Transformation|GetActorLocation))
  (Rendering|Debug|DrawDebugLine (Variables|Default|GetLastPosition) _returnvalue (CallFunction|GetTraceColor) (Variables|Default|GetTraceDuration) 0.0)
  (Variables|Default|SetLastPosition _returnvalue))

(event EventBeginPlay
  (Utilities|Time|SetTimerbyFunctionName self "Update" 0.01 true) ; Temp
)

(fn ConstructionScript
  (Variables|Default|SetLastPosition (Transformation|GetActorLocation))
  (Variables|Default|SetInitialVelocity (Transformation|GetVelocity)))

(fn DeterminePenetration
  (params (ImpactVelocity :type Vector%20%28by%20ref%29))
  (if (> (Math|Vector|VectorLength ImpactVelocity) 1.6e+03)
    (return)))

(fn ComputeExitLocation
  (params (ImpactVelocity :type Vector%20%28by%20ref%29) (HitResult :type Hit%20Result%20Structure%20%28by%20ref%29))
  (bind _location (Collision|BreakHitResult HitResult))
  (Collision|MultiSphereTraceForObjects (+ (* (Math|Vector|Normalize ImpactVelocity) 5e+02) _location) _location 0.0 (Variables|Default|GetObjectsToDetect) false 0 "None"))

(fn GetTraceColor
  (bind _projectilemovement (Variables|Default|GetProjectileMovement))
  (bind _velocity (Variables|/Script/Engine.MovementComponent|GetVelocity _projectilemovement))
  (bind _initialspeed (Variables|/Script/Engine.ProjectileMovementComponent|GetInitialSpeed _projectilemovement))
  (bind _returnvalue (Math|Vector|VectorLength _velocity))
  (bind _returnvalue_2 (/ _returnvalue _initialspeed))
  (if (> _returnvalue_2 0.75)
    (return (Math|Color|Lerp(LinearColor) "(R=1.000000,G=1.000000,B=0.000000,A=1.000000)" "(R=1.000000,G=0.000000,B=0.000000,A=1.000000)" (* (- _returnvalue_2 0.75) 4.0)))
    (elif (> _returnvalue_2 0.5)
      (return (Math|Color|Lerp(LinearColor) "(R=0.000000,G=1.000000,B=0.000000,A=1.000000)" "(R=1.000000,G=1.000000,B=0.000000,A=1.000000)" (* (- _returnvalue_2 0.5) 4.0)))
      (elif (> _returnvalue_2 0.25)
        (return (Math|Color|Lerp(LinearColor) "(R=0.000000,G=0.000000,B=1.000000,A=1.000000)" "(R=0.000000,G=1.000000,B=0.000000,A=1.000000)" (* (- _returnvalue_2 0.25) 4.0)))
        (else
          (return (Math|Color|Lerp(LinearColor) "(R=1.000000,G=1.000000,B=1.000000,A=1.000000)" "(R=0.000000,G=0.000000,B=1.000000,A=1.000000)" (* _returnvalue_2 4.0))))))))

(fn GetNewSpeed
  (params (Hit :type Hit%20Result%20Structure%20%28by%20ref%29) (ExitLocation :type Vector%20%28by%20ref%29))
  (return (Math|Float|Sqrt (Math|Float|%(Float) (- (* 0.5 (Variables|Default|GetMass) (Math|Vector|VectorLengthSquared ExitLocation)) (* (Math|Vector|VectorLength (- ExitLocation (.Location (Collision|BreakHitResult Hit)))) 3e+04)) (* 0.5 (Variables|Default|GetMass))))))