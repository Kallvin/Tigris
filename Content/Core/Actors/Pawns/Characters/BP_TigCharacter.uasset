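; BP_TigCharacter is a character Blueprint that handles health, fall damage and death, with a special death case for its player subclass.
; Any damage lowers clamped health, and hard landings apply falling-type damage scaled by vertical speed.
; At zero health it disables controller input, stops movement and destroys itself after a delay.
; A temporary branch quits the game first when the actor is the player character.
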(event Custom|Death
  ;[1 1 1] Damage
  ;;[1 1 1] Death
  (Variables|State|SetbIsDead true)
  (Input|DisableInput (Pawn|GetController) 0)
  (Components|Movement|StopMovementImmediately (Variables|Character|GetCharacterMovement))
  (CallFunction|COut "Death" "Actor has died, self destruction emminent." "(R=1.000000,G=0.000000,B=0.000000,A=1.000000)" false)
  (Utilities|FlowControl|Delay 1e+01)
  ;[1 1 1] Temp
  (bind _asbp_tig_character_player (Utilities|Casting|CastToBP_TigCharacter_Player self)
    (:then
      (bind _asplayer_controller (Utilities|Casting|CastToPlayerController (Pawn|GetController _asbp_tig_character_player)))
      (Game|QuitGame _asplayer_controller "Quit" false)
      (Actor|DestroyActor))
    (:CastFailed
      (Actor|DestroyActor))))

(event EventBeginPlay
  (CallFunction|COut "BeginPlay" "Checking in." "(R=0.000000,G=1.000000,B=0.000000,A=1.000000)" false))

(event Game|Damage|EventAnyDamage
  (params (Damage :type Float%20%28single-precision%29) (DamageType :type Damage%20Type%20Object%20Reference) (InstigatedBy :type Controller%20Object%20Reference) (DamageCauser :type Actor%20Object%20Reference))
  ;[1 1 1] Damage
  (bind _output_get (Variables|Attributes|SetHealthCurrent (Math|Float|Clamp(Float) (- (Variables|Attributes|GetHealthCurrent) Damage) 0.0 (Variables|Attributes|GetHealthMax))))
  (if (Math|Float|NearlyEqual(Float) _output_get 0.0 0.0001)
    (CallFunction|Death)))

(event Game|Damage|EventPointDamage
  (params (Damage :type Float%20%28single-precision%29) (DamageType :type Damage%20Type%20Object%20Reference) (HitLocation :type Vector :default "0, 0, 0") (HitNormal :type Vector :default "0, 0, 0") (HitComponent :type Primitive%20Component%20Object%20Reference) (BoneName :type Name :default "None") (ShotFromDirection :type Vector :default "0, 0, 0") (InstigatedBy :type Controller%20Object%20Reference) (DamageCauser :type Actor%20Object%20Reference) (HitInfo :type Hit%20Result%20Structure%20%28by%20ref%29))
  ;[1 1 1] Damage
)

(event Game|Damage|EventRadialDamage
  (params (DamageReceived :type Float%20%28single-precision%29) (DamageType :type Damage%20Type%20Object%20Reference) (Origin :type Vector :default "0, 0, 0") (HitInfo :type Hit%20Result%20Structure%20%28by%20ref%29) (InstigatedBy :type Controller%20Object%20Reference) (DamageCauser :type Actor%20Object%20Reference))
  ;[1 1 1] Damage
)

(event EventOnLanded
  (params (Hit :type Hit%20Result%20Structure%20%28by%20ref%29))
  (bind _returnvalue (Transformation|GetVelocity))
  (bind _returnvalue_2 (Math|Float|Absolute(Float) (.z _returnvalue)))
  (bind _returnvalue_3 (Math|Float|NormalizetoRange _returnvalue_2 8e+02 1.6e+03))
  (bind _returnvalue_4 (Math|Float|Clamp(Float) _returnvalue_3))
  ;[1 1 1] Damage
  ;;[1 1 1] Fall Damage
  (if (> _returnvalue_4 0.0)
    (Game|Damage|ApplyDamage self (* _returnvalue_4 4.0) 0 (.HitActor (Collision|BreakHitResult Hit)) "/Game/Core/DamageTypes/BP_TigDamageType_Falling.BP_TigDamageType_Falling_C")))

(fn ConstructionScript)