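; BP_TigGameInstance is the game instance that handles menus, multiplayer sessions and player save data.
; Interface events show cached or new menu widgets, create a session that opens the lobby, join or destroy sessions, and store the selected character.
; Network, travel and session failures feed a shared error popup.
; Player info persists through BP_TigSaveGame in one slot, with a check that loads existing data or creates the save.
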(event Custom|ToggleDebugPrintToScreen
  ;[1 1 1] Debug
  (bind _isa (Utilities|FlowControl|FlipFlop)
    (:A
      _)
    (:B
      _))
  (bind _output_get (Variables|Debug|SetbDebugPrintToScreen (not _isa)))
  (CallFunction|COut "ToggleDebugPrintToScreen" (Utilities|Text|FormatText "Toggling: {Bool}" _output_get) "(R=0.000000,G=1.000000,B=1.000000,A=1.000000)" false))

(event Custom|ToggleDebugPrintToLog
  ;[1 1 1] Debug
  (bind _isa (Utilities|FlowControl|FlipFlop)
    (:A
      _)
    (:B
      _))
  (bind _output_get (Variables|Debug|SetbDebugPrintToLog (not _isa)))
  (CallFunction|COut "ToggleDebugPrintToLog" (Utilities|Text|FormatText "Toggling: {Bool}" _output_get) "(R=0.000000,G=1.000000,B=1.000000,A=1.000000)" false))

(event EventInit
  (CallFunction|COut "Initialize" "Checking in." "(R=0.000000,G=1.000000,B=0.000000,A=1.000000)" false))

(event EventHandleNetworkError
  (params (FailureType :type ENetworkFailure%20Enum :default "NetDriverAlreadyExists") (bIsServer :type Boolean))
  ;[1 1 1] Net Errors
  (if bIsServer
    _
    (else
      _))
  (CallFunction|CreateErrorMessage (Utilities|Text|ToText(String) (CallFunction|NetErrortoString FailureType))))

(event EventHandleTravelError
  (params (FailureType :type ETravelFailure%20Enum :default "NoLevel"))
  ;[1 1 1] Net Errors
  (CallFunction|CreateErrorMessage (Utilities|Text|ToText(String) (CallFunction|TravelErrortoString FailureType))))

(event EventSavePlayerInfo
  (params (PlayerInfoToSave :type F%20Player%20Info%20Structure))
  (Variables|Save|GetSaveGameRef
    (:then
      _)
    (:else
      (bind _returnvalue (SaveGame|CreateSaveGameObject "/Game/Core/SaveGames/BP_TigSaveGame.BP_TigSaveGame_C"))
      (bind _output_get (Variables|Save|SetSaveGameRef _returnvalue))))
  (Default|StorePlayerInfo _output_get PlayerInfoToSave)
  (SaveGame|SaveGametoSlot (Variables|Save|GetSaveGameRef) "PlayerSave"))

(event EventSaveGameCheck
  (CallFunction|InstanceSaveGameCheck))

(event Custom|SaveGame
  ;[1 1 1] SaveGame - Saves the player information.
  (CallFunction|COut "SaveGame" "Deprecated, please use SavePlayerInfo." "(R=0.000000,G=1.000000,B=1.000000,A=1.000000)" false)
  (CallFunction|SavePlayerInfo (Variables|Save|GetPlayers%20Info)))

(event EventStoreSelectedCharacter
  (params (SelectedCharacterID :type Integer))
  ;[1 1 1] StoreSelectedCharacter - Not sure why this is stored here instead of in the LobbyGameMode or elsewhere entirely as it's relevency is questionable anywhere outside of the lobby character selection screen.
  (bind _output_get (Variables|Session|SetSelected%20Character%20ID SelectedCharacterID))
  (if (!= _output_get 0)
    (Variables|Default|SetSelectedCharacterClass (Utilities|Array|Get(acopy) (Variables|Default|GetCharactersToSelect) (Variables|Session|GetSelected%20Character%20ID)))))

(event EventJoinServer
  (params (SessionToJoin :type Blueprint%20Session%20Result%20Structure))
  ;[1 1 1] JoinServer
  (CallFunction|ShowLoadingScreen)
  (|JoinSession (Game|GetPlayerController 0) SessionToJoin
    (:OnFailure
      (CallFunction|CreateErrorMessage "Failed to join server: Please try again!"))))

(event EventDestroySessionCaller
  (params (PlayerController :type Player%20Controller%20Object%20Reference))
  ;[1 1 1] DestroySessionCaller
  (|DestroySession PlayerController
    (:OnFailure
      (CallFunction|CreateErrorMessage "Failed to destroy session: Please try again!"))))

(event EventShowHostMenu
  ;[1 1 1] Host Menu
  (bind _hostmenu (Variables|Widgets|GetHostMenu)
    (:then
      (UserInterface|Viewport|AddtoViewport _hostmenu 0)
      (Widget|SetVisibility _hostmenu "Visible") ; Show Host Menu.
    )
    (:else
      (bind _returnvalue (UserInterface|CreateWidget "/Game/Core/Widgets/Menu/WBP_HostMenu.WBP_HostMenu_C" (Game|GetPlayerController 0)))
      (bind _output_get (Variables|Widgets|SetHostMenu _returnvalue))
      (UserInterface|Viewport|AddtoViewport _output_get 0))))

(event EventShowServerMenu
  ;[1 1 1] ServerMenu
  (bind _returnvalue (UserInterface|CreateWidget "/Game/Core/Widgets/Menu/WBP_ServerMenu.WBP_ServerMenu_C" (Game|GetPlayerController 0)))
  (UserInterface|Viewport|AddtoViewport _returnvalue 0))

(event EventShowOptionsMenu
  ;[1 1 1] OptionsMenu
  (Variables|Default|GetWBP%20Options%20Menu
    (:then
      (Variables|Default|GetWBP%20Options%20Menu
        (:then
          (Widget|SetVisibility (Variables|Default|GetWBP%20Options%20Menu) "Visible"))
        (:else)))
    (:else
      (bind _aswbp_main_menu (Utilities|Casting|CastToWBP_MainMenu (Variables|Widgets|GetMainMenu))
        (:then
          (Variables|Default|SetWBP%20Options%20Menu (Variables|/Game/Core/Widgets/Menu/Main/WBP_MainMenu.WBP_MainMenu_C|GetWBP_OptionsMenu _aswbp_main_menu)))
        (:CastFailed
          (CallFunction|COut "ShowOptionsMenu" "WBP_MainMenu" "(R=0.000000,G=1.000000,B=1.000000,A=1.000000)" true))))))

(event EventLaunchLobby
  (params (NumberOfPlayers :type Integer) (bEnableLAN? :type Boolean) (ServerName :type Text))
  ;[1 1 1] LaunchLobby
  (Variables|Session|SetMaxPlayers NumberOfPlayers)
  (Variables|Session|SetServerName ServerName)
  (CallFunction|ShowLoadingScreen)
  (|Session (Game|GetPlayerController 0) (Variables|Session|GetMaxPlayers) bEnableLAN?
    (:OnSuccess
      ;;[1 1 1] Open Lobby Level using the game mode instead?
      (Game|OpenLevel(byObjectReference) "/Game/Art/Maps/L_Lobby.L_Lobby"))
    (:OnFailure
      (CallFunction|CreateErrorMessage "Failed to create session: Please try again."))))

(fn GetSetGameMode
  (bind _asbp_tig_menu_game_mode (Utilities|Casting|CastToBP_TigMenuGameMode (Game|GetGameMode))
    (:then
      (Variables|References|SetAs%20BP%20Tig%20Menu%20Game%20Mode _asbp_tig_menu_game_mode))
    (:CastFailed
      (CallFunction|COut "BeginPlay" "BP_TigGameMode" "(R=0.000000,G=1.000000,B=0.000000,A=1.000000)" true)))
  (return))

(fn CreateErrorMessage
  (params (Message :type Text))
  (bind _errorwindow (Variables|Widgets|GetErrorWindow)
    (:then
      (if (UserInterface|Viewport|IsinViewport _errorwindow)
        (Widget|RemovefromParent _errorwindow)
        (bind _returnvalue (UserInterface|CreateWidget "/Game/Core/Widgets/Menu/WBP_ErrorWindow.WBP_ErrorWindow_C" (Game|GetPlayerController 0) :!label _label))
        (bind _output_get (Variables|Widgets|SetErrorWindow _returnvalue))
        (UserInterface|Viewport|AddtoViewport _output_get 1)))
    (:else
      (goto _label)))
  (Default|SetMessage (.AsWBP%20Error%20Window (Utilities|Casting|CastToWBP_ErrorWindow (Variables|Widgets|GetErrorWindow))) Message)
  (return))

(fn GetSetHUD
  (bind _asbp_tig_hud (Utilities|Casting|CastToBP_TigHUD (HUD|GetHUD (Game|GetPlayerController 0)))
    (:then
      (Variables|References|SetAs%20BP%20Tig%20HUD _asbp_tig_hud))
    (:CastFailed
      (CallFunction|COut "ShowMainMenu" "BP_TigHUD" "(R=0.000000,G=1.000000,B=1.000000,A=1.000000)" true)))
  (return))

(fn NetErrortoString
  (params (FailureType :type ENetworkFailure%20Enum :default "NetDriverAlreadyExists"))
  (switch Utilities|FlowControl|Switch|SwitchonENetworkFailure FailureType
    (:NetDriverAlreadyExists
      (LocalVariables|SetLocal_ErrorString "Error: Lost Connection to Host." :!label _label))
    (:NetDriverCreateFailure
      (goto _label))
    (:NetDriverListenFailure
      (goto _label))
    (:ConnectionLost
      (goto _label))
    (:ConnectionTimeout
      (LocalVariables|SetLocal_ErrorString "Error: Connection Timed Out."))
    (:FailureReceived
      (goto _label))
    (:OutdatedClient
      (goto _label))
    (:OutdatedServer
      (goto _label))
    (:PendingConnectionFailure
      (goto _label)))
  (return (LocalVariables|GetLocal_ErrorString)))

(fn TravelErrortoString
  (params (FailureType :type ETravelFailure%20Enum :default "NoLevel"))
  (return (Utilities|String|Append "Error: Failed to Travel -- " (Utilities|String|EnumtoString FailureType))))

(fn InstanceSaveGameCheck
  (bind _returnvalue (SaveGame|DoesSaveGameExist "PlayerSave"))
  (if _returnvalue
    (CallFunction|LoadPlayerInfo)
    (return true)
    (else
      (CallFunction|SavePlayerInfo (Variables|Save|GetPlayers%20Info))
      (return false))))

(fn CustomGameInstanceRef
  (return self))

(fn LoadPlayerInfo
  (bind _returnvalue (SaveGame|LoadGamefromSlot "PlayerSave"))
  (bind _asbp_tig_save_game (Utilities|Casting|CastToBP_TigSaveGame _returnvalue)
    (:then
      (bind _output_get (Variables|Save|SetPlayers%20Info (Variables|/Game/Core/SaveGames/BP_TigSaveGame.BP_TigSaveGame_C|GetPlayerInfo _asbp_tig_save_game)))
      (return _output_get))
    (:CastFailed
      (CallFunction|COut "LoadPlayerInfo" "BP_TigSaveGame" "(R=0.000000,G=1.000000,B=1.000000,A=1.000000)" true))))

(fn ShowLoadingScreen
  ;[1 1 1] LoadingScreen
  (bind _loadingscreen (Variables|Widgets|GetLoadingScreen)
    (:then
      (Widget|SetVisibility _loadingscreen "Visible") ; Show Loading Screen
      (UserInterface|Viewport|AddtoViewport _loadingscreen 0))
    (:else
      (bind _returnvalue (UserInterface|CreateWidget "/Game/Core/Widgets/Menu/WBP_LoadingScreen.WBP_LoadingScreen_C" (Game|GetPlayerController 0)))
      (Variables|Widgets|SetLoadingScreen _returnvalue)))
  (return))

(fn ShowMainMenu
  (bind _returnvalue (Game|GetPlayerController 0))
  ;[1 1 1] ShowMainMenu
  (bind _mainmenu (Variables|Widgets|GetMainMenu)
    (:then
      (UserInterface|Viewport|AddtoViewport _mainmenu 0)
      (Widget|SetVisibility _mainmenu "Visible") ; Show Main Menu.
    )
    (:else
      ;;[1 1 1] Create a new main menu.
      (bind _returnvalue_2 (UserInterface|CreateWidget "/Game/Core/Widgets/Menu/Main/WBP_MainMenu.WBP_MainMenu_C" _returnvalue))
      (bind _output_get (Variables|Widgets|SetMainMenu _returnvalue_2))
      (UserInterface|Viewport|AddtoViewport _output_get 0)))
  (Variables|/Script/Engine.PlayerController|SetbShowMouseCursor _returnvalue true)
  (return))